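; Game mode for a Snake game that keeps food in play and reacts to the snake's death.
; On Tick it checks the food spawner and, once no spawned actors remain, has it spawn its configured count again.
; The SnakeIsDead event calls the HUD reference to show the death menu.
; Both paths act only when their reference is valid, and neither reference is assigned in this Blueprint's graphs.
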(event EventTick
  (params (DeltaSeconds :type Float%20%28single-precision%29))
  (bind _foodspawner (Variables|Food|GetFoodSpawner))
  (bind _foodspawner_2 (Variables|Food|GetFoodSpawner))
  (bind _spawnedactors (Variables|/Script/SnakeGame_Homework.ActorSpawner|GetSpawnedActors _foodspawner_2))
  (bind _returnvalue (Utilities|Array|Length _spawnedactors))
  (bind _returnvalue_2 (== _returnvalue 0))
  (Utilities|IsValid _foodspawner_2
    (:Is%20Valid
      (if _returnvalue_2
        (Class|ActorSpawner|SpawnActors _foodspawner (Variables|/Script/SnakeGame_Homework.ActorSpawner|GetActorsCount _foodspawner) _returnvalue_2)))))

(event EventSnakeIsDead
  (bind _hudreference (Variables|HUD|GetHudReference))
  (Utilities|IsValid _hudreference
    (:Is%20Valid
      (Default|ShowDiedMenuEvent _hudreference false))))

(fn ConstructionScript)